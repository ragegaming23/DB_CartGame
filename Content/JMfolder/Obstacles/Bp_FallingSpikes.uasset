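; Falling spike trap obstacle that drops three spikes when the player enters its trigger, and can damage and slow the player.
; The trigger starts a short timer, which enables physics on the spikes and removes the activation component if the player is still in range.
; Three hit boxes share a DoOnce with a delayed reset, damaging the player and lowering walk speed on any overlap, with no speed restore here.
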(event OnComponentBeginOverlap(Box)
  (params (OverlappedComponent :type Primitive%20Component%20Object%20Reference) (OtherActor :type Actor%20Object%20Reference) (OtherComp :type Primitive%20Component%20Object%20Reference) (OtherBodyIndex :type Integer) (bFromSweep :type Boolean) (SweepResult :type Hit%20Result%20Structure%20%28by%20ref%29))
  (Utilities|FlowControl|DoOnce false :!label _label
    (:Completed
      (Game|Damage|ApplyDamage (Game|GetPlayerCharacter 0) 1.0 0 0)
      (Variables|/Script/Engine.CharacterMovementComponent|SetMaxWalkSpeed (Variables|/Script/Engine.Character|GetCharacterMovement (Game|GetPlayerCharacter 0)) (Variables|Default|Getdecrease%20speed))
      (Utilities|FlowControl|Delay 5.0)
      (goto _label Reset))))

(event OnComponentBeginOverlap(Box1)
  (params (OverlappedComponent :type Primitive%20Component%20Object%20Reference) (OtherActor :type Actor%20Object%20Reference) (OtherComp :type Primitive%20Component%20Object%20Reference) (OtherBodyIndex :type Integer) (bFromSweep :type Boolean) (SweepResult :type Hit%20Result%20Structure%20%28by%20ref%29))
  (Utilities|FlowControl|DoOnce false :!label _label
    (:Completed
      (Game|Damage|ApplyDamage (Game|GetPlayerCharacter 0) 1.0 0 0)
      (Variables|/Script/Engine.CharacterMovementComponent|SetMaxWalkSpeed (Variables|/Script/Engine.Character|GetCharacterMovement (Game|GetPlayerCharacter 0)) (Variables|Default|Getdecrease%20speed))
      (Utilities|FlowControl|Delay 5.0)
      (goto _label Reset))))

(event OnComponentBeginOverlap(SpikeFall_Activate)
  (params (OverlappedComponent :type Primitive%20Component%20Object%20Reference) (OtherActor :type Actor%20Object%20Reference) (OtherComp :type Primitive%20Component%20Object%20Reference) (OtherBodyIndex :type Integer) (bFromSweep :type Boolean) (SweepResult :type Hit%20Result%20Structure%20%28by%20ref%29))
  (if (== OtherActor (Game|GetPlayerCharacter 0))
    (Variables|Default|SetEnterSpikeRange true)
    (bind _returnvalue (Utilities|Time|SetTimerbyEvent (delegate Custom|PlatformBreak) 0.1))))

(event OnComponentEndOverlap(SpikeFall_Activate)
  (params (OverlappedComponent :type Primitive%20Component%20Object%20Reference) (OtherActor :type Actor%20Object%20Reference) (OtherComp :type Primitive%20Component%20Object%20Reference) (OtherBodyIndex :type Integer))
  (if (== OtherActor (Game|GetPlayerCharacter 0))
    (Variables|Default|SetEnterSpikeRange false)))

(event OnComponentBeginOverlap(Box2)
  (params (OverlappedComponent :type Primitive%20Component%20Object%20Reference) (OtherActor :type Actor%20Object%20Reference) (OtherComp :type Primitive%20Component%20Object%20Reference) (OtherBodyIndex :type Integer) (bFromSweep :type Boolean) (SweepResult :type Hit%20Result%20Structure%20%28by%20ref%29))
  (Utilities|FlowControl|DoOnce false :!label _label
    (:Completed
      (Game|Damage|ApplyDamage (Game|GetPlayerCharacter 0) 1.0 0 0)
      (Variables|/Script/Engine.CharacterMovementComponent|SetMaxWalkSpeed (Variables|/Script/Engine.Character|GetCharacterMovement (Game|GetPlayerCharacter 0)) (Variables|Default|Getdecrease%20speed))
      (Utilities|FlowControl|Delay 5.0)
      (goto _label Reset))))

(event Custom|PlatformBreak
  (if (Variables|Default|GetEnterSpikeRange)
    (Physics|SetSimulatePhysics (Variables|Default|GetSpike) true)
    (Components|DestroyComponent (Variables|Default|GetSpikeFall_Activate)))
  (Utilities|Time|ClearandInvalidateTimerbyHandle (stale OnComponentBeginOverlap(SpikeFall_Activate) _returnvalue)))

(fn ConstructionScript)