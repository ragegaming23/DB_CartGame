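; Falling platform obstacle that drops once the player character steps into its trigger.
; Begin and end overlap on the trigger set an in-range flag, with entry also starting a very short timer.
; If the player is still in range when the timer fires, the platform starts simulating physics and the trigger is destroyed, so it falls only once.
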(event OnComponentBeginOverlap(PlatformFall_Trigger)
  (params (OverlappedComponent :type Primitive%20Component%20Object%20Reference) (OtherActor :type Actor%20Object%20Reference) (OtherComp :type Primitive%20Component%20Object%20Reference) (OtherBodyIndex :type Integer) (bFromSweep :type Boolean) (SweepResult :type Hit%20Result%20Structure%20%28by%20ref%29))
  (if (== OtherActor (Game|GetPlayerCharacter 0))
    (Variables|Default|SetEnterPlatformRange true)
    (bind _returnvalue (Utilities|Time|SetTimerbyEvent (delegate Custom|PlatformBreak) 0.01))))

(event OnComponentEndOverlap(PlatformFall_Trigger)
  (params (OverlappedComponent :type Primitive%20Component%20Object%20Reference) (OtherActor :type Actor%20Object%20Reference) (OtherComp :type Primitive%20Component%20Object%20Reference) (OtherBodyIndex :type Integer))
  (if (== OtherActor (Game|GetPlayerCharacter 0))
    (Variables|Default|SetEnterPlatformRange false)))

(event Custom|PlatformBreak
  (if (Variables|Default|GetEnterPlatformRange)
    (Physics|SetSimulatePhysics (Variables|Default|GetPlatform) true)
    (Components|DestroyComponent (Variables|Default|GetPlatformFall_Trigger)))
  (Utilities|Time|ClearandInvalidateTimerbyHandle (stale OnComponentBeginOverlap(PlatformFall_Trigger) _returnvalue)))

(event EventBeginPlay)

(event Collision|EventActorBeginOverlap
  (params (OtherActor :type Actor%20Object%20Reference)))

(event EventTick
  (params (DeltaSeconds :type Float%20%28single-precision%29)))

(fn ConstructionScript)