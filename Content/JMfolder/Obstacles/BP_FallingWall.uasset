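; BP_FallingWall is an obstacle wall that falls by physics when the player enters its trigger.
; The trigger overlap starts a short timer, which enables wall physics and destroys the trigger if the player is still inside.
; A separate box damages and slows the player, gated by a resettable DoOnce with a delay; speed is never restored here.
; An arrow component supplies the wall's attach transform.
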(event OnComponentBeginOverlap(ActivateWall_Trigger)
  (params (OverlappedComponent :type Primitive%20Component%20Object%20Reference) (OtherActor :type Actor%20Object%20Reference) (OtherComp :type Primitive%20Component%20Object%20Reference) (OtherBodyIndex :type Integer) (bFromSweep :type Boolean) (SweepResult :type Hit%20Result%20Structure%20%28by%20ref%29))
  (if (== OtherActor (Game|GetPlayerCharacter 0))
    (Variables|Default|SetEnterWallRange true)
    (bind _returnvalue (Utilities|Time|SetTimerbyEvent (delegate Custom|PlatformBreak) 0.1))))

(event OnComponentEndOverlap(ActivateWall_Trigger)
  (params (OverlappedComponent :type Primitive%20Component%20Object%20Reference) (OtherActor :type Actor%20Object%20Reference) (OtherComp :type Primitive%20Component%20Object%20Reference) (OtherBodyIndex :type Integer))
  (if (== OtherActor (Game|GetPlayerCharacter 0))
    (Variables|Default|SetEnterWallRange false)))

(event OnComponentBeginOverlap(Box)
  (params (OverlappedComponent :type Primitive%20Component%20Object%20Reference) (OtherActor :type Actor%20Object%20Reference) (OtherComp :type Primitive%20Component%20Object%20Reference) (OtherBodyIndex :type Integer) (bFromSweep :type Boolean) (SweepResult :type Hit%20Result%20Structure%20%28by%20ref%29))
  (bind _returnvalue (Game|GetPlayerCharacter 0))
  (if (== OtherActor _returnvalue)
    (Utilities|FlowControl|DoOnce false :!label _label
      (:Completed
        (Game|Damage|ApplyDamage _returnvalue 1.0 0 0)
        (Variables|/Script/Engine.CharacterMovementComponent|SetMaxWalkSpeed (Variables|/Script/Engine.Character|GetCharacterMovement (Game|GetPlayerCharacter 0)) (Variables|Default|GetDecreaseSpeed))
        (Utilities|FlowControl|Delay 5.0)
        (goto _label Reset)))))

(event Custom|PlatformBreak
  (if (Variables|Default|GetEnterWallRange)
    (Physics|SetSimulatePhysics (Variables|Default|GetWall) true)
    (Components|DestroyComponent (Variables|Default|GetActivateWall_Trigger)))
  (Utilities|Time|ClearandInvalidateTimerbyHandle (stale OnComponentBeginOverlap(ActivateWall_Trigger) _returnvalue)))

(fn ConstructionScript)

(fn GetWallAttatchPoint
  (return (Transformation|GetWorldTransform (Variables|Default|GetArrow))))