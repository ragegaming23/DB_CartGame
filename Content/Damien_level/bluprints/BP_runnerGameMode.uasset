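; Game mode for a runner level that builds an endless floor out of spawned tiles.
; BeginPlay lays the starting tiles, chaining each new BP_floor_00 to the attach point returned by the previous one.
; ExtendFloor adds a tile and destroys the oldest once the array exceeds NumberOfTiles plus two.
; AddWall and AddSpikes chain falling hazards the same way, but are called only from an unreachable sequence.
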(event EventBeginPlay
  (for _index (range 0 (- (Variables|Default|Getnumber%20of%20tiles) 1))
    (CallFunction|AddFloor)))

(fn ConstructionScript)

(fn AddFloor
  (bind _returnvalue (Game|SpawnActorfromClass "/Game/Damien_level/bluprints/BP_floor_00.BP_floor_00_C" (Variables|Default|Getfloor%20attatch%20point) "Undefined" "MultiplyWithRoot" 0 0))
  (bind _returnvalue_2 (Default|GetAttatchPoint _returnvalue))
  (Variables|Default|Setfloor%20attatch%20point _returnvalue_2)
  (Utilities|Array|Add (Variables|Default|Getfloor%2000%20tiles) _returnvalue))

(fn ExtendFloor
  (bind _floor_00_tiles (Variables|Default|Getfloor%2000%20tiles))
  (bind _output (Utilities|Array|Get(acopy) _floor_00_tiles))
  (CallFunction|AddFloor)
  (if (> (Utilities|Array|Length (Variables|Default|Getfloor%2000%20tiles)) (+ (Variables|Default|Getnumber%20of%20tiles) 2))
    (Actor|DestroyActor _output)
    (Utilities|Array|RemoveItem _floor_00_tiles _output)))

(fn AddWall
  (bind _returnvalue (Game|SpawnActorfromClass "/Game/JMfolder/Obstacles/BP_FallingWall.BP_FallingWall_C" (Variables|Default|GetWall%20Attach%20point) "Undefined" "MultiplyWithRoot" 0 0))
  (bind _returnvalue_2 (Default|GetWallAttatchPoint _returnvalue))
  (Variables|Default|SetWall%20Attach%20point _returnvalue_2)
  (Utilities|Array|Add (Variables|Default|GetWall%20Spawn) _returnvalue))

(fn AddSpikes
  (bind _returnvalue (Game|SpawnActorfromClass "/Game/JMfolder/Obstacles/Bp_FallingSpikes.Bp_FallingSpikes_C" (Variables|Default|GetSpike%20Attatch%20point) "Undefined" "MultiplyWithRoot" 0 0))
  (bind _returnvalue_2 (Default|GetSpikeAttatchPoint _returnvalue))
  (Variables|Default|SetSpike%20Attatch%20point _returnvalue_2)
  (Utilities|Array|Add (Variables|Default|GetSpike%20spawn) _returnvalue))